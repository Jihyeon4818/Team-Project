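; BP_MonsterSpawner is an actor that spawns a set quantity of AI monsters, one at a time, once play begins.
; Each monster appears at the Scene component's location with a fixed rotation, receives MonsterTarget as its StartTarget, and gets its default controller.
; A self-calling Spawn event with delays paces the spawns a few seconds apart, decrementing Quantity until none remain.
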(event `self.ReceiveBeginPlay`
  (`self.Spawn`))

(event `Spawn`
  (`KismetSystemLibrary.Delay` 0.1)
  (if (> (`self.Quantity`) 0)
    (bind _returnvalue (`|SpawnActorFromClass` "/Game/Book/YeChan/Monster/AIMonster.AIMonster_C" (`KismetMathLibrary.MakeTransform` (`SceneComponent.K2_GetComponentLocation` (`self.Scene`)) (struct :`Yaw` 90.0)) "Undefined" "OverrideRootScale" null (`self.MonsterTarget`) null))
    (`Pawn.SpawnDefaultController` _returnvalue)
    (set `self.Quantity` (- (`self.Quantity`) 1))
    (`KismetSystemLibrary.Delay` 3.0)
    (`self.Spawn`)))

(fn `UserConstructionScript`)